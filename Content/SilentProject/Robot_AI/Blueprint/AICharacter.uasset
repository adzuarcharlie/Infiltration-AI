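; Robot AI character that registers with a shared helper on spawn and reacts to perceiving the player.
; On detection, it clears controller orders, notifies the helper and writes player, spotted time and, for sight, last-seen location to the Blackboard.
; On loss, it clears the player, zeroes the cooldown timer and notifies the helper; hearing is only stubbed.
; GetPerceptionLockRot exposes the mesh's PerceptionSocket world location and rotation.
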(event `self.ReceiveBeginPlay`
  (bind _returnvalue (`self.GetHelper`))
  (`AIHelper.AddEntity` _returnvalue self))

(event `self.AIPerception.OnTargetPerceptionUpdated`
  (params (Actor :type "Actor Object Reference") (Stimulus :type "AIStimulus Structure"))
  (bind (_age _expirationage _strength _stimuluslocation _receiverlocation _tag _bsuccessfullysensed) (break `AIStimulus` Stimulus))
  (bind _returnvalue (`AIBlueprintHelperLibrary.GetBlackboard` null))
  (bind _returnvalue_2 (`KismetStringLibrary.Conv_StringToName` "PlayerCharacter"))
  (bind _assp_00character (cast `SP_00Character` Actor))
  (bind _returnvalue_3 (`self.GetHelper`))
  ;[1 1 1] the event is called when the player enters and when he quits the perception, so we chech if it is successfully sensed (true means he enters the perception, false means he quits)
  (if _bsuccessfullysensed
    (bind _assp_aicontroller (cast `SP_AIController` (`self.GetController`))
      (:`then`
        ;[1 1 1] remove orders that need to be (orders that have the Deleted When PLayer Is Spotted bool set to true)
        (`SP_AIController.ClearOrders` _assp_aicontroller)
        (`AIHelper.EntitySeesPlayer` _returnvalue_3 self)
        (`BlackboardComponent.SetValueAsFloat` _returnvalue (`KismetStringLibrary.Conv_StringToName` "TimePlayerWasSpotted") (`KismetSystemLibrary.GetGameTimeInSeconds`))
        (`BlackboardComponent.SetValueAsObject` _returnvalue _returnvalue_2 _assp_00character)
        ;[0.1 0.1 1] this part is not used for now because we only implemented sight, but this is how to do if we want to implement hearing and other senses and modify the behaviour according to which sense is touched
        (bind _returnvalue_4 (`AIPerceptionSystem.GetSenseClassForStimulus` Stimulus))
        (bind _returnvalue_5 (`KismetSystemLibrary.GetClassDisplayName` _returnvalue_4))
        (if (`KismetStringLibrary.EqualEqual_StrStr` "AISense_Sight" _returnvalue_5)
          (`BlackboardComponent.SetValueAsVector` _returnvalue (`KismetStringLibrary.Conv_StringToName` "LastSeen") _stimuluslocation)
          (elif (`KismetStringLibrary.EqualEqual_StrStr` "AISense_Hearing" _returnvalue_5)
            _)))
      (:`CastFailed`
        (`KismetSystemLibrary.PrintString` "ERROR : COULD NOT CAST AI CONTROLLER")))
    (else
      ;[1 1 1] Player is lost
      (`BlackboardComponent.SetValueAsObject` _returnvalue _returnvalue_2 null)
      (`BlackboardComponent.SetValueAsFloat` _returnvalue (`KismetStringLibrary.Conv_StringToName` "CooldownTimer") 0.0)
      (`AIHelper.EntityLostPlayer` _returnvalue_3 self))))

(fn `GetPerceptionLockRot`
  (returns (OutLocation :type "Vector Structure") (OutRotation :type "Rotator Structure"))
  (return (.location (`SceneComponent.GetSocketTransform` (`self.Mesh`) "PerceptionSocket" "RTS_World")) (.rotation (`SceneComponent.GetSocketTransform` (`self.Mesh`) "PerceptionSocket" "RTS_World"))))

(fn `UserConstructionScript`)